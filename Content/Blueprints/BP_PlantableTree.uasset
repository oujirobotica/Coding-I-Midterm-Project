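; BP_PlantableTree is a tree actor that enlarges its static mesh shortly after play begins.
; BeginPlay passes through a DoN node with a random count and a short delay, then Grow adds a random amount to the mesh's scale.
; An always-true branch then sets collision to physics-only and prints a debug message, so the loop back never runs and the tree grows only once.
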(event `self.ReceiveBeginPlay`
  (bind _counter (`/Engine/EditorBlueprintResources/StandardMacros.Do N` (`KismetMathLibrary.RandomIntegerInRange` 2 5) :!label _label)
    (:`Exit`
      (`KismetSystemLibrary.Delay` 0.5)
      (`self.Grow`)
      (if true
        (`PrimitiveComponent.SetCollisionEnabled` (`self.SM_Generic_Tree_02`) "PhysicsOnly")
        (`KismetSystemLibrary.PrintText` "Set Col. Enabled")
        (else
          (goto _label))))))

(event `Grow`
  (`SceneComponent.SetRelativeScale3D` (`self.SM_Generic_Tree_02`) (+ (`SceneComponent.RelativeScale3D` (`self.SM_Generic_Tree_02`)) (`KismetMathLibrary.RandomFloatInRange` 1.0 2.0))))

(fn `UserConstructionScript`)