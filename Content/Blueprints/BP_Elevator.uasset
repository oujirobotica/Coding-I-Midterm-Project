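; BP_Elevator is an elevator actor that rises when a third-person character holding at least one elevator key overlaps it.
; On overlap it checks the character's key count, then switches on the BP_ElevatorLight found by class lookup.
; A timeline then lerps the elevator's relative Z between fixed heights, feeding world X and Y back in as relative coordinates.
; Debug text reports each step, including a missing key.
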(event `self.ReceiveBeginPlay`)

(event `self.ReceiveActorBeginOverlap`
  (params (OtherActor :type "Actor Object Reference"))
  (bind (_returnvalue_x _returnvalue_y) (`KismetMathLibrary.BreakVector` (`self.K2_GetActorLocation`)))
  (bind _asbp_third_person_character (cast `/Game/ThirdPerson/Blueprints/BP_ThirdPersonCharacter` OtherActor))
  (`KismetSystemLibrary.PrintText` "Player is touching Elevator!")
  (if (>= (`/Game/ThirdPerson/Blueprints/BP_ThirdPersonCharacter.TotalElevatorKeys` _asbp_third_person_character) 1)
    (`KismetSystemLibrary.PrintText` "Player has elevator key!")
    (bind _returnvalue (`GameplayStatics.GetActorOfClass` "/Game/Blueprints/BP_ElevatorLight.BP_ElevatorLight_C"))
    (bind _asbp_elevator_light (cast `/Game/Blueprints/BP_ElevatorLight` _returnvalue))
    (`/Game/Blueprints/BP_ElevatorLight.ElevatorOn` _asbp_elevator_light) ; Access Elevator light
    (`KismetSystemLibrary.PrintText` "Elevator is on!")
    (bind (_direction _elevator_up_down) (`Timeline|Timeline`)
      (:`Update`
        (`self.K2_SetActorRelativeLocation` (`KismetMathLibrary.MakeVector` _returnvalue_x _returnvalue_y (`KismetMathLibrary.Lerp` 0.0 100.0 _elevator_up_down)))))
    (else
      (`KismetSystemLibrary.PrintText` "Player has no elevator key!"))))

(fn `UserConstructionScript`)