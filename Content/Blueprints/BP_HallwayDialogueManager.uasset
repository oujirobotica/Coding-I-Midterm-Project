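; BP_HallwayDialogueManager shows lines from a Dialogue array one at a time, presumably for a hallway sequence.
; It creates a W_Dialogue widget on BeginPlay and keeps it for reuse.
; Each DisplayNextLine call prints the current line, shows it in the widget for a few seconds and advances the index.
; Past the last line, it restarts only if ShouldRepeatText is set, otherwise it shows nothing.
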(event `self.ReceiveBeginPlay`
  (bind _returnvalue (`|CreateWidget` "/Game/Widgets/W_Dialogue.W_Dialogue_C")) ; create widget
  (set `self.Dialogue Widget` _returnvalue) ; Promote to Variable
)

(event `DisplayNextLine`
  (bind _dialogue_widget (`self.Dialogue Widget`))
  (bind _output (`|GetArrayItem` (`self.Dialogue`) (`self.Index`)))
  (if (>= (`self.Index`) (`KismetArrayLibrary.Array_Length` (`self.Dialogue`)))
    (if (`self.ShouldRepeatText`)
      (set `self.Index` 0)
      (`KismetSystemLibrary.PrintText` _output true true (struct :`R` 1.0 :`G` 0.627934 :`A` 1.0) 5.0 :!label _label)
      (`TextBlock.SetText` (`/Game/Widgets/W_Dialogue.Textblock0` (`self.Dialogue Widget`)) _output)
      (`|ExecutionSequence`
        (:`then_0`
          (`UserWidget.AddToViewport` _dialogue_widget 0) ; add dialogue to the view
          (`KismetSystemLibrary.Delay` 4.0) ; wait 5 seconds
          (`Widget.RemoveFromParent` _dialogue_widget) ; remove the dialogue from the view
        )
        (:`then_1`
          (`/Engine/EditorBlueprintResources/StandardMacros.IncrementInt` (`self.Index`)) ; Increment Int\nto add 1 to our index
        )))
    (else
      (goto _label))))

(fn `UserConstructionScript`)