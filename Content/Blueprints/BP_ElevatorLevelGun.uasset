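; Elevator level gun that watches for the player along its barrel and, when triggered, advances dialogue rather than shooting.
; Every Tick it runs a debug-drawn 1000-unit forward line trace, flagging any hit on the third-person character.
; A two-second Delay on Tick repeatedly calls FireGun, which, if flagged, calls the DialogueManager's next line, prints a message and clears the flag.
; Bullet spawning and impulse nodes are present but disconnected.
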(event `self.ReceiveTick`
  (params (DeltaSeconds :type "Float (single-precision)"))
  (bind _cylind_001_cylinder_001 (`self.cylind_001_Cylinder_001`))
  (bind _returnvalue (`SceneComponent.K2_GetComponentLocation` _cylind_001_cylinder_001))
  (bind (_outhit _returnvalue_2) (`KismetSystemLibrary.LineTraceSingle` :`Start` _returnvalue :`End` (+ _returnvalue (* (`KismetMathLibrary.GetForwardVector` (`SceneComponent.K2_GetComponentRotation` _cylind_001_cylinder_001)) 1000.0)) :`TraceChannel` "TraceTypeQuery2" :`DrawDebugType` "ForOneFrame"))
  (`|ExecutionSequence`
    (:`then_0`
      (bind (_bblockinghit _binitialoverlap _time _distance _location _impactpoint _normal _impactnormal _physmat _hitactor) (`GameplayStatics.BreakHitResult` _outhit))
      (cast `/Game/ThirdPerson/Blueprints/BP_ThirdPersonCharacter` _hitactor)
      (set `self.HitPlayerRecently` true))
    (:`then_1`
      (`KismetSystemLibrary.PrintText` (`KismetTextLibrary.Conv_StringToText` (`KismetSystemLibrary.GetDisplayName` _hitactor)) _returnvalue_2)
      (`KismetSystemLibrary.Delay` 2.0)
      (`self.Fire Gun`))))

(event `Fire Gun`
  (if (`self.HitPlayerRecently`)
    (`/Game/Blueprints/BP_BaseDialogueManager_V2.DisplayNextLine` (`self.dialogueManager`))
    (`KismetSystemLibrary.PrintText` "is Firing!")
    (set `self.HitPlayerRecently` false)))

(fn `UserConstructionScript`)