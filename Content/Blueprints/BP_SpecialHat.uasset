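; BP_SpecialHat is a wearable pickup hat that spawns stars when its primary action fires.
; On overlap with BP_ThirdPersonCharacter, it stores the player, calls TryToPickupItem with itself and attaches to the head socket of the player's mesh, keeping world rotation.
; PrimaryAction prints a debug message and spawns a BP_Star at the hat's transform.
; Drop is an empty stub.
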(event `self.ReceiveActorBeginOverlap`
  (params (OtherActor :type "Actor Object Reference"))
  (bind _asbp_third_person_character (cast `/Game/ThirdPerson/Blueprints/BP_ThirdPersonCharacter` OtherActor))
  (set `self.player` _asbp_third_person_character)
  (`self.Pickup`))

(event `/Game/Blueprints/BPI_Item.Drop`)

(event `/Game/Blueprints/BPI_Item.PrimaryAction`
  (`KismetSystemLibrary.PrintText` "Click sensed!")
  (`|SpawnActorFromClass` "/Game/Blueprints/BP_Star.BP_Star_C" (`self.GetTransform` self) "Undefined" "MultiplyWithRoot" null null))

(event `/Game/Blueprints/BPI_Item.Pickup`
  (bind _player (`self.player`))
  (`/Game/ThirdPerson/Blueprints/BP_ThirdPersonCharacter.Try To Pickup Item` _player self)
  (`self.K2_AttachToComponent` (`Character.Mesh` _player) "head" "SnapToTarget" "KeepWorld" "KeepRelative"))

(fn `UserConstructionScript`)